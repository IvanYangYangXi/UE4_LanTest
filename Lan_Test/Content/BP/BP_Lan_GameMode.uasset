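; LAN multiplayer GameMode that switches all players between first- and third-person characters and broadcasts a test event to clients.
; PostLogin collects each PlayerController in an array that the other logic loops over.
; Each switch event destroys the current pawn, spawns the new character at the first PlayerStart found and possesses it.
; BT_EventTest_SendToClient fans out server-side by calling BTEventTestReplicatedToOwningClient on each BP_Lan_Contraller.
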(event Custom|ChangeCharacterToFP
  ;[1 1 1] 切换角色
  (for _array_element (Variables|Default|GetLoginPlayerController)
    ;;[1 1 1] 清除原来的角色
    (Actor|DestroyActor (Pawn|GetControlledPawn _array_element))
    ;;[1 1 1] 获取player Start 的位置
    (bind _outactors (Actor|GetAllActorsOfClass "/Script/Engine.PlayerStart"))
    (bind _returnvalue (Game|SpawnActorfromClass "/Game/FirstPersonBP/Blueprints/FirstPersonCharacter.FirstPersonCharacter_C" (Transformation|GetActorTransform (Utilities|Array|Get(acopy) _outactors)) "Undefined" 0 0))
    (Pawn|Possess _array_element _returnvalue)))

(event Custom|ChangeCharacterToTP
  ;[1 1 1] 切换角色
  (for _array_element (Variables|Default|GetLoginPlayerController)
    (Actor|DestroyActor (Pawn|GetControlledPawn _array_element))
    ;;[1 1 1] 获取player Start 的位置
    (bind _outactors (Actor|GetAllActorsOfClass "/Script/Engine.PlayerStart"))
    (bind _returnvalue (Game|SpawnActorfromClass "/Game/ThirdPersonBP/Blueprints/ThirdPersonCharacter.ThirdPersonCharacter_C" (Transformation|GetActorTransform (Utilities|Array|Get(acopy) _outactors)) "Undefined" 0 0))
    (Pawn|Possess _array_element _returnvalue)))

(event EventBeginPlay)

(event EventTick
  (params (DeltaSeconds :type Float%20%28single-precision%29)))

(event EventPostLogin
  (params (NewPlayer :type Player%20Controller%20Object%20Reference))
  (Utilities|Array|Add (Variables|Default|GetLoginPlayerController) NewPlayer))

(fn ConstructionScript)

(fn BTEventTestSendtoClient
  ;[1 1 1] 服务端收到此事件调用请求时，群发给每一个客户端要执行的事件
  (for _array_element (Variables|Default|GetLoginPlayerController)
    (bind _asbp_lan_contraller (Utilities|Casting|CastToBP_Lan_Contraller _array_element))
    (Default|BTEventTestReplicatedtoOwningClient _asbp_lan_contraller)))